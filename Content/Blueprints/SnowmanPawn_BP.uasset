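; SnowmanPawn_BP is a player-input pawn that slides the snowman along the world X or Y axis.
; The MoveX and MoveY axis events store clamped input and flag which axis is active.
; Tick applies delta-time-scaled movement via SetActorLocation without sweep, with X taking priority so it never moves diagonally.
; Each moving tick also calls GetAllActorsOfClass, but its result is unused.
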(event `self.ReceiveTick`
  (params (DeltaSeconds :type "Float (single-precision)"))
  (bind _speed_multiplier (`self.SPEED_MULTIPLIER`))
  (bind (_x _y _z) (`KismetMathLibrary.BreakVector3f` (`self.K2_GetActorLocation`)))
  (bind (_x_2 _y_2 _z_2) (`KismetMathLibrary.BreakVector3f` (`self.K2_GetActorLocation`)))
  (if (`self.alongX`)
    (`GameplayStatics.GetAllActorsOfClass` null)
    (bind _output_get (set `self.locationX` _x))
    (bind _output_get_2 (set `self.locationX` (+ _output_get (* (`self.movementX`) DeltaSeconds _speed_multiplier))))
    (`self.K2_SetActorLocation` (`KismetMathLibrary.MakeVector` _output_get_2 _y _z))
    (elif (`self.alongY`)
      (`GameplayStatics.GetAllActorsOfClass` null)
      (bind _output_get_3 (set `self.locationY` _y_2))
      (bind _output_get_4 (set `self.locationY` (+ _output_get_3 (* _speed_multiplier DeltaSeconds (`self.movementY`)))))
      (`self.K2_SetActorLocation` (`KismetMathLibrary.MakeVector` _x_2 _output_get_4 _z_2)))))

(event `InputAxis|MoveX`
  (params (AxisValue :type "Float (single-precision)"))
  (bind _output_get (set `self.movementX` (`KismetMathLibrary.FClamp` AxisValue -1.0)))
  (set `self.alongX` (!= _output_get 0.0)))

(event `InputAxis|MoveY`
  (params (AxisValue :type "Float (single-precision)"))
  (bind _output_get (set `self.movementY` (`KismetMathLibrary.FClamp` AxisValue -1.0)))
  (set `self.alongY` (!= _output_get 0.0)))

(fn `UserConstructionScript`)